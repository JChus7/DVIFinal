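; BP_ky_magicCircle1 is a magic circle effect actor that serves as a spawn point for skeleton enemies.
; Its Spawn event picks a sword, archer or mage skeleton from a type index and spawns it as AI.
; Archers and mages appear at random points inside the AreaSpawn box, while swordsmen appear at its world location.
; The construction script passes the Color variable to the Fx component's color parameter.
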(event `Spawn`
  (params (TipoSpawn :type Integer))
  (bind _areaspawn (`self.AreaSpawn`))
  (bind _returnvalue (`SceneComponent.K2_GetComponentLocation` _areaspawn))
  (bind _returnvalue_2 (`KismetMathLibrary.RandomPointInBoundingBox` _returnvalue (`BoxComponent.GetScaledBoxExtent` _areaspawn)))
  ;[1 1 1] Seleccion del tipo de enemigo
  (switch `int` TipoSpawn
    (:`0`
      ;[1 1 1] Spawn del enemigo
      (`AIBlueprintHelperLibrary.SpawnAIFromClass` "/Game/SkeletonCrew/Skeleton_Swordsman/BB_EsqueletoEspada.BB_EsqueletoEspada_C" null _returnvalue))
    (:`1`
      (`AIBlueprintHelperLibrary.SpawnAIFromClass` "/Game/SkeletonCrew/Skeleton_Archer/BB_EsqueletoArquero.BB_EsqueletoArquero_C" null _returnvalue_2))
    (:`2`
      (`AIBlueprintHelperLibrary.SpawnAIFromClass` "/Game/SkeletonCrew/Skeleton_Mage/BB_EsqueletoMago.BB_EsqueletoMago_C" null _returnvalue_2))))

(fn `UserConstructionScript`
  (`parent.UserConstructionScript`)
  (`ParticleSystemComponent.SetVectorParameter` (`self.fx`) "color" (`KismetMathLibrary.Conv_LinearColorToVector` (`self.color`))))